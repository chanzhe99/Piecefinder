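; BP_Puzzle_Fuzebox is a puzzle fuse box that is solved by inserting a fuse key at normal scale.
; On overlap with its collision box, a BP_Key_Fuze near unit scale snaps to the FuzeSocket on the box.
; It then clears the player finder character's targeting state, marks itself solved and immediately quits the game.
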(event OnComponentBeginOverlap(CollisionBox)
  (params (OverlappedComponent :type Primitive%20Component%20Object%20Reference) (OtherActor :type Actor%20Object%20Reference) (OtherComp :type Primitive%20Component%20Object%20Reference) (OtherBodyIndex :type Integer) (bFromSweep :type Boolean) (SweepResult :type Hit%20Result%20Structure%20%28by%20ref%29))
  (if (not (Variables|Default|GetisSolved))
    (bind _asbp_key_fuze (Utilities|Casting|CastToBP_Key_Fuze OtherActor))
    (if (Math|Vector|Equal(Vector) (Transformation|GetActorScale3D _asbp_key_fuze) "1.000000,1.000000,1.000000" 0.1)
      (Transformation|AttachComponentToComponent OtherActor (Variables|Default|GetBox) "FuzeSocket" "SnapToTarget" "SnapToTarget" "SnapToTarget" true)
      (bind _asbp_finder_character (Utilities|Casting|CastToBP_FinderCharacter (Game|GetPlayerCharacter 0)))
      (Variables|/Game/Blueprints/BP_FinderCharacter.BP_FinderCharacter_C|SetHitObject _asbp_finder_character 0)
      (Variables|/Game/Blueprints/BP_FinderCharacter.BP_FinderCharacter_C|SetTargetInFrame _asbp_finder_character false)
      (Variables|Default|SetisSolved true)
      (Game|QuitGame (Game|GetPlayerController 0) "Quit" false))))

(fn ConstructionScript)