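; BP_SoundTrigger plays the sounds in its AudioSample array back to back as 2D audio, starting at BeginPlay.
; A hand-built latent loop plays the clip at Index, delays for its duration, then increments Index and repeats, gated by a LastAudioClipCompleted flag.
; The loop has no end-of-array check.
; An unconnected ForEach version remains in the graph, and CustomLoop is empty.
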(event EventBeginPlay
  (if (Variables|Default|GetLastAudioClipCompleted) :!label _label
    (Variables|Default|SetLastAudioClipCompleted false)
    (Audio|PlaySound2D (Utilities|Array|Get(acopy) (Variables|Default|GetAudioSample) (Variables|Default|GetIndex)) 1.0 1.0 0.0 0 0)
    (Utilities|FlowControl|Delay (Variables|/Script/Engine.SoundBase|GetDuration (Utilities|Array|Get(acopy) (Variables|Default|GetAudioSample) (Variables|Default|GetIndex))))
    (Variables|Default|SetLastAudioClipCompleted true)
    (Variables|Default|SetIndex (+ (Variables|Default|GetIndex) 1))
    (goto _label)))

(fn ConstructionScript)