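; First-person character with a raisable viewfinder frame that grabs and drops objects using a Superliminal-style forced-perspective resize.
; Capture, with the frame up, line-traces from the view to store the hit actor, distance, scale and rotation offset, or releases the held one.
; Tick eases the frame, holds the object on the view ray and re-traces past it, scaling it by current over starting distance.
; Scene-capture and centering logic is disconnected.
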(event Custom|MoveRight
  (params (AxisValue :type Float%20%28single-precision%29))
  (Pawn|Input|AddMovementInput (Transformation|GetActorRightVector) AxisValue false))

(event Custom|LookRight
  (params (AxisValue :type Float%20%28single-precision%29))
  (Pawn|Input|AddControllerYawInput AxisValue))

(event Custom|Capture
  (if (Variables|Default|GetIsFrameUp)
    (if (Variables|Default|GetTargetInFrame)
      (Variables|Default|SetHitObject 0)
      (Variables|Default|SetTargetInFrame false)
      (Variables|Default|SetObjectMovedToCenter false)
      (else
        (CallFunction|TraceLinefromView)))))

(event Custom|MoveForward
  (params (AxisValue :type Float%20%28single-precision%29))
  (Pawn|Input|AddMovementInput (Transformation|GetActorForwardVector) AxisValue false))

(event Custom|RaiseFrame
  (Variables|Default|SetIsFrameUp (not (Variables|Default|GetIsFrameUp))))

(event Custom|LookUp
  (params (AxisValue :type Float%20%28single-precision%29))
  (Pawn|Input|AddControllerPitchInput AxisValue))

(event Collision|EventActorBeginOverlap
  (params (OtherActor :type Actor%20Object%20Reference)))

(event EventBeginPlay
  (Transformation|SetRelativeLocation (Variables|Default|GetFrame) (Variables|Default|GetFrameDownPosition) false false)
  (Rendering|ClearRenderTarget2D "/Game/Materials/RT_Capture.RT_Capture"))

(event EventTick
  (params (DeltaSeconds :type Float%20%28single-precision%29))
  (bind (_outlocation _outrotation) (Actor|GetActorEyesViewPoint))
  (bind (_outlocation_2 _outrotation_2) (Actor|GetActorEyesViewPoint))
  (Transformation|SetWorldLocationAndRotation (Variables|Default|GetScene) _outlocation_2 _outrotation_2 false false)
  (CallFunction|LerpFrameLocation)
  (if (Variables|Default|GetTargetInFrame)
    (bind _output_get (Variables|Default|SetLocationOfObject (+ _outlocation (* (Math|Rotator|GetRotationXVector _outrotation) (Variables|Default|GetTargetDistance)))))
    (Transformation|SetActorLocationAndRotation (Variables|Default|GetHitObject) _output_get (Math|Rotator|CombineRotators (Variables|Default|GetObjectRotationOffset) (Pawn|GetControlRotation :!class /Script/Engine.Pawn)))
    (CallFunction|TraceCheckforWall)
    (Transformation|SetActorScale3D (Variables|Default|GetHitObject) (Math|Vector|Lerp(Vector) (Transformation|GetActorScale3D (Variables|Default|GetHitObject)) (* (Variables|Default|GetObjectScale) (/ (Variables|Default|GetTargetDistance) (Variables|Default|GetStartingDistance))) (* (Utilities|Time|GetWorldDeltaSeconds) 1e+02)))))

(fn ConstructionScript)

(fn LerpFrameLocation
  (bind _frame (Variables|Default|GetFrame))
  (Transformation|SetRelativeLocation _frame (Math|Vector|Lerp(Vector) (Variables|/Script/Engine.SceneComponent|GetRelativeLocation _frame) (Math|Vector|SelectVector (Variables|Default|GetFrameUpPosition) (Variables|Default|GetFrameDownPosition) (Variables|Default|GetIsFrameUp)) (* (Utilities|Time|GetWorldDeltaSeconds) (Variables|Default|GetLerpSpeed))) false false))

(fn TraceLinefromView
  (bind (_outlocation _outrotation) (Actor|GetActorEyesViewPoint))
  (bind (_outhit _returnvalue) (Collision|LineTraceByChannel _outlocation (+ _outlocation (* (Math|Rotator|GetRotationXVector _outrotation) 1e+04)) "TraceTypeQuery1" false 0 "ForDuration" true "(R=1.000000,G=0.000000,B=0.000000,A=1.000000)" "(R=0.000000,G=1.000000,B=0.000000,A=1.000000)" 1.0))
  (bind _output_get (Variables|Default|SetTargetInFrame _returnvalue))
  (if _output_get
    (bind _output_get_2 (Variables|Default|SetStartingDistance (.Distance (Collision|BreakHitResult _outhit))))
    (Variables|Default|SetTargetDistance _output_get_2)
    (bind _output_get_3 (Variables|Default|SetHitObject (.HitActor (Collision|BreakHitResult _outhit))))
    (bind _output_get_4 (Variables|Default|SetObjectRotationOffset (Math|Conversions|RotationFromXVector (- (Transformation|GetActorLocation) (Transformation|GetActorLocation _output_get_3)))))
    (Variables|Default|SetObjectScale (Transformation|GetActorScale3D _output_get_3))))

(fn TraceCheckforWall
  (bind (_outlocation _outrotation) (Actor|GetActorEyesViewPoint))
  (bind _outhit (Collision|LineTraceByChannel _outlocation (+ _outlocation (* (Math|Rotator|GetRotationXVector _outrotation) 1e+04)) "TraceTypeQuery1" false (Utilities|Array|MakeArray (Variables|Default|GetHitObject)) "ForOneFrame" true "(R=1.000000,G=0.000000,B=0.000000,A=1.000000)" "(R=0.000000,G=1.000000,B=0.000000,A=1.000000)" 1.0))
  (Variables|Default|SetTargetDistance (.Distance (Collision|BreakHitResult _outhit))))