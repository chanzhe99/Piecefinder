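; BP_FinderController is the player controller for the Finder character.
; On BeginPlay it casts and caches the controlled pawn as BP_FinderCharacter, then creates the UI_HUD widget and adds it to the viewport.
; It forwards move, look and jump inputs to that character, with left click calling Capture and right click press calling RaiseFrame.
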(event EventBeginPlay
  (bind _asbp_finder_character (Utilities|Casting|CastToBP_FinderCharacter (Pawn|GetControlledPawn)))
  (Variables|Default|SetFinder _asbp_finder_character)
  (bind _returnvalue (UserInterface|CreateWidget "/Game/Blueprints/UI/UI_HUD.UI_HUD_C" self))
  (UserInterface|Viewport|AddtoViewport _returnvalue 0))

(event Input|ActionEvents|InputActionRightClick
  (params (Key :type Key%20Structure :default "None"))
  (:Pressed
    (Default|RaiseFrame (Variables|Default|GetFinder))))

(event Input|ActionEvents|InputActionJump
  (params (Key :type Key%20Structure :default "None"))
  (:Pressed
    (Character|Jump (Variables|Default|GetFinder))))

(event Input|ActionEvents|InputActionLeftClick
  (params (Key :type Key%20Structure :default "None"))
  (:Pressed
    (Default|Capture (Variables|Default|GetFinder))))

(event Input|AxisEvents|InputAxisMoveForward
  (params (AxisValue :type Float%20%28single-precision%29))
  (Default|MoveForward (Variables|Default|GetFinder) AxisValue))

(event Input|AxisEvents|InputAxisMoveRight
  (params (AxisValue :type Float%20%28single-precision%29))
  (Default|MoveRight (Variables|Default|GetFinder) AxisValue))

(event Input|AxisEvents|InputAxisLookUp
  (params (AxisValue :type Float%20%28single-precision%29))
  (Default|LookUp (Variables|Default|GetFinder) AxisValue))

(event Input|AxisEvents|InputAxisLookRight
  (params (AxisValue :type Float%20%28single-precision%29))
  (Default|LookRight (Variables|Default|GetFinder) AxisValue))

(fn ConstructionScript)